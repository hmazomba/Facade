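; Character stand-in in the SceneCaptures folder that displays equipped gear on its own skeletal mesh, likely for a captured character view.
; On BeginPlay it passes itself to the player's CH_Character, and its EquipItem and UnEquipItem events attach or destroy items by slot.
; Attach helpers spawn armor or weapons onto sockets named in their info structs, but only destroy an already valid item without spawning its replacement.
; Weapon helpers disable the recorder's collision, not the weapon's.
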(event EventBeginPlay
  (bind _asch_character (Utilities|Casting|CastToCH_Character (Game|GetPlayerCharacter 0)))
  (Class|BPIRecorderCom|PassReference(Message) _asch_character self))

(event EventEquipItem
  (params (ItemInfo :type F%20Item%20Info%20Structure))
  (CallFunction|AttachItem ItemInfo))

(event EventUnEquipItem
  (params (ItemInfo :type F%20Item%20Info%20Structure))
  (CallFunction|DetachItem ItemInfo))

(fn ConstructionScript)

(fn AttachItem
  (params (ItemInfo :type F%20Item%20Info%20Structure))
  (bind (_itemclass _itemslot) (Utilities|Struct|BreakFItemInfo ItemInfo))
  (switch Utilities|FlowControl|Switch|SwitchonESlotType _itemslot
    (:NewEnumerator1
      (CallFunction|AttachArmorPiece (Variables|Default|GetHeadItem) _itemclass))
    (:NewEnumerator2
      (CallFunction|AttachArmorPiece (Variables|Default|GetTorsoItem) _itemclass))
    (:NewEnumerator3
      (CallFunction|AttachArmorPiece (Variables|Default|GetArmsItem) _itemclass))
    (:NewEnumerator4
      (CallFunction|AttachArmorPiece (Variables|Default|GetLegsItem) _itemclass))
    (:NewEnumerator5
      (CallFunction|AttachArmorPiece (Variables|Default|GetFeetItem) _itemclass))
    (:NewEnumerator6
      (CallFunction|AttachPrimaryRight (Variables|Default|GetPrimaryRightHand) _itemclass))
    (:NewEnumerator7
      (CallFunction|AttachPrimaryLeft (Variables|Default|GetPrimaryLeftHand) _itemclass))
    (:NewEnumerator8
      (CallFunction|AttachSecondaryRight (Variables|Default|GetSecondaryRightHand) _itemclass))
    (:NewEnumerator9
      (CallFunction|AttachSecondaryLeft (Variables|Default|GetSecondaryLeftHand) _itemclass))
    (:NewEnumerator10
      (CallFunction|AttachArmorPiece (Variables|Default|GetAmulet) _itemclass))))

(fn AttachArmorPiece
  (params (Item :type BP%20Base%20Item%20Object%20Reference) (ItemClass :type BP%20Base%20Item%20Class%20Reference))
  (Utilities|IsValid Item
    (:Is%20Valid
      (Actor|DestroyActor Item))
    (:Is%20Not%20Valid
      (bind _returnvalue (Game|SpawnActorfromClass ItemClass (Transformation|GetActorTransform) "AlwaysSpawn" 0 0))
      (Utilities|FlowControl|Sequence
        (:then_0
          (return _returnvalue))
        (:then_1
          (bind _asbp_base_armor (Utilities|Casting|CastToBP_BaseArmor _returnvalue))
          (Transformation|AttachComponentToComponent _asbp_base_armor (Variables|Default|GetSkeletalMesh) (Utilities|Struct|BreakFArmorInfo (Variables|/Game/Core/BP/Interactables/Armor/BP_BaseArmor.BP_BaseArmor_C|GetArmorInfo _asbp_base_armor)) "KeepRelative" "KeepRelative" "KeepRelative" true)
          (Collision|SetActorEnableCollision _asbp_base_armor false))))))

(fn DetachItem
  (params (ItemInfo :type F%20Item%20Info%20Structure))
  (switch Utilities|FlowControl|Switch|SwitchonESlotType (Utilities|Struct|BreakFItemInfo ItemInfo)
    (:NewEnumerator1
      (Actor|DestroyActor (Variables|Default|GetHeadItem)))
    (:NewEnumerator2
      (Actor|DestroyActor (Variables|Default|GetTorsoItem)))
    (:NewEnumerator3
      (Actor|DestroyActor (Variables|Default|GetArmsItem)))
    (:NewEnumerator4
      (Actor|DestroyActor (Variables|Default|GetLegsItem)))
    (:NewEnumerator5
      (Actor|DestroyActor (Variables|Default|GetFeetItem)))
    (:NewEnumerator6
      (Actor|DestroyActor (Variables|Default|GetPrimaryRightHand)))
    (:NewEnumerator7
      (Actor|DestroyActor (Variables|Default|GetPrimaryLeftHand)))
    (:NewEnumerator8
      (Actor|DestroyActor (Variables|Default|GetSecondaryRightHand)))
    (:NewEnumerator9
      (Actor|DestroyActor (Variables|Default|GetSecondaryLeftHand)))
    (:NewEnumerator10
      (Actor|DestroyActor (Variables|Default|GetAmulet)))))

(fn AttachPrimaryLeft
  (params (Item :type BP%20Base%20Item%20Object%20Reference) (ItemClass :type BP%20Base%20Item%20Class%20Reference))
  (Utilities|IsValid Item
    (:Is%20Valid
      (Actor|DestroyActor Item))
    (:Is%20Not%20Valid
      (bind _returnvalue (Game|SpawnActorfromClass ItemClass (Transformation|GetActorTransform) "AlwaysSpawn" 0 0))
      (Utilities|FlowControl|Sequence
        (:then_0
          (return _returnvalue))
        (:then_1
          (bind _asbp_base_weapon (Utilities|Casting|CastToBP_BaseWeapon _returnvalue))
          (Transformation|AttachComponentToComponent _asbp_base_weapon (Variables|Default|GetSkeletalMesh) (Utilities|Struct|BreakFWeaponInfo (Variables|/Game/Core/BP/Interactables/Weapons/BP_BaseWeapon.BP_BaseWeapon_C|GetWeaponInfo _asbp_base_weapon)) "KeepRelative" "KeepRelative" "KeepRelative" true)
          (Collision|SetActorEnableCollision false))))))

(fn AttachPrimaryRight
  (params (Item :type BP%20Base%20Item%20Object%20Reference) (ItemClass :type BP%20Base%20Item%20Class%20Reference))
  (Utilities|IsValid Item
    (:Is%20Valid
      (Actor|DestroyActor Item))
    (:Is%20Not%20Valid
      (bind _returnvalue (Game|SpawnActorfromClass ItemClass (Transformation|GetActorTransform) "AlwaysSpawn" 0 0))
      (Utilities|FlowControl|Sequence
        (:then_0
          (return _returnvalue))
        (:then_1
          (bind _asbp_base_weapon (Utilities|Casting|CastToBP_BaseWeapon _returnvalue))
          (Transformation|AttachComponentToComponent _asbp_base_weapon (Variables|Default|GetSkeletalMesh) (Utilities|Struct|BreakFWeaponInfo (Variables|/Game/Core/BP/Interactables/Weapons/BP_BaseWeapon.BP_BaseWeapon_C|GetWeaponInfo _asbp_base_weapon)) "KeepRelative" "KeepRelative" "KeepRelative" true)
          (Collision|SetActorEnableCollision false))))))

(fn AttachSecondaryLeft
  (params (Item :type BP%20Base%20Item%20Object%20Reference) (ItemClass :type BP%20Base%20Item%20Class%20Reference))
  (Utilities|IsValid Item
    (:Is%20Valid
      (Actor|DestroyActor Item))
    (:Is%20Not%20Valid
      (bind _returnvalue (Game|SpawnActorfromClass ItemClass (Transformation|GetActorTransform) "AlwaysSpawn" 0 0))
      (Utilities|FlowControl|Sequence
        (:then_0
          (return _returnvalue))
        (:then_1
          (bind _asbp_base_weapon (Utilities|Casting|CastToBP_BaseWeapon _returnvalue))
          (Transformation|AttachComponentToComponent _asbp_base_weapon (Variables|Default|GetSkeletalMesh) (Utilities|Struct|BreakFWeaponInfo (Variables|/Game/Core/BP/Interactables/Weapons/BP_BaseWeapon.BP_BaseWeapon_C|GetWeaponInfo _asbp_base_weapon)) "KeepRelative" "KeepRelative" "KeepRelative" true)
          (Collision|SetActorEnableCollision false))))))

(fn AttachSecondaryRight
  (params (Item :type BP%20Base%20Item%20Object%20Reference) (ItemClass :type BP%20Base%20Item%20Class%20Reference))
  (Utilities|IsValid Item
    (:Is%20Valid
      (Actor|DestroyActor Item))
    (:Is%20Not%20Valid
      (bind _returnvalue (Game|SpawnActorfromClass ItemClass (Transformation|GetActorTransform) "AlwaysSpawn" 0 0))
      (Utilities|FlowControl|Sequence
        (:then_0
          (return _returnvalue))
        (:then_1
          (bind _asbp_base_weapon (Utilities|Casting|CastToBP_BaseWeapon _returnvalue))
          (Transformation|AttachComponentToComponent _asbp_base_weapon (Variables|Default|GetSkeletalMesh) (Utilities|Struct|BreakFWeaponInfo (Variables|/Game/Core/BP/Interactables/Weapons/BP_BaseWeapon.BP_BaseWeapon_C|GetWeaponInfo _asbp_base_weapon)) "KeepRelative" "KeepRelative" "KeepRelative" true)
          (Collision|SetActorEnableCollision false))))))